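; BP_PoopSmear is an interactable poop smear decal whose opacity reflects its smear amount.
; Construction creates a dynamic decal material, rotates the actor and applies that opacity.
; Collider overlap only attempts a FloorSection cast when DamageGiven is set.
; Disconnected logic would decrease GameState level health by smear amount and the highest overlapping floor multiplier, then set DamageGiven, but it never runs.
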(event `self.Collider.OnComponentBeginOverlap`
  (params (OverlappedComponent :type "PrimitiveComponent Object Reference") (OtherActor :type "Actor Object Reference") (OtherComp :type "PrimitiveComponent Object Reference") (OtherBodyIndex :type Integer) (bFromSweep :type Boolean) (SweepResult :type "HitResult Structure (by ref)"))
  (if (`self.DamageGiven`)
    (cast `FloorSection` OtherActor)))

(fn `SetOpacity`
  (params (Opacity :type "Float (double-precision)" :default 1.0))
  (`MaterialInstanceDynamic.SetScalarParameterValue` (`self.MI_DecalMaterial`) "Opacity" Opacity))

(fn `UserConstructionScript`
  (bind _returnvalue (`KismetMaterialLibrary.CreateDynamicMaterialInstance` "/Game/KittyCatastrophe/MaterialLibrary/M_PoopSmear_Decal.M_PoopSmear_Decal" "PoopSmear_Decal"))
  (bind _output_get (set `self.MI_DecalMaterial` _returnvalue))
  (`DecalComponent.SetDecalMaterial` (`self.PoopSmear`) _output_get)
  (`self.K2_SetActorRelativeRotation` (struct :`Pitch` 90.0))
  (`self.SetOpacity` (`self.SMEAR_AMOUNT`)))