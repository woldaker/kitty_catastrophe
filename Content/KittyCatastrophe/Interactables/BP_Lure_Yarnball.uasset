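; Yarn ball lure interactable that expires after a limited lifespan, flickering as a warning before it is destroyed.
; A looping one-second timer counts down TimeToLive, starts the fade-out at a threshold and destroys the actor at zero.
; The fade is a timeline whose Flicker events briefly toggle Yarn visibility.
; ResetLifespan cancels the fade and restores the countdown, and GetPhysicsBody exposes Yarn as the physics body.
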(event `self.ReceiveBeginPlay`
  (`KismetSystemLibrary.K2_SetTimer` null "DecrementLifeSpanTimer" 1.0 true))

(event `FadeOut`
  (bind _yarn (`self.Yarn`))
  ;[1 1 1] Fades out before getting destroyed.
  (`Timeline|FadeOutTimeline` :!via `PlayFromStart` :!label _label
    (:`Flicker`
      (`SceneComponent.SetVisibility` _yarn false false)
      (`KismetSystemLibrary.Delay` 0.1)
      (`SceneComponent.SetVisibility` _yarn true false))))

(event `StopFadeOut`
  ;[1 1 1] Fades out before getting destroyed.
  (goto _label :!via `Stop`))

(fn `DecrementLifeSpanTimer`
  (bind _result (`/Engine/EditorBlueprintResources/StandardMacros.DecrementInt` (`self.TimeToLive`))
    (:`  `
      (if (<= _result 0)
        (`self.K2_DestroyActor`)
        (elif (== _result (`self.FADE_AT_TIME`))
          (`self.FadeOut`))))))

(fn `GetPhysicsBody`
  (returns (PhysicsBody :type "StaticMeshComponent Object Reference"))
  (return (`self.Yarn`)))

(fn `ResetLifespan`
  (`self.StopFadeOut`)
  (set `self.TimeToLive` (`self.LIFESPAN`))
  (`SceneComponent.SetVisibility` (`self.Yarn`) true false))

(fn `UserConstructionScript`
  (set `self.TimeToLive` (`self.LIFESPAN`)))