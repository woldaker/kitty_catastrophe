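; BP_Poop is a physics-driven poop interactable that damages level health through floor sections and can be stepped in by the kitty.
; On overlapping a floor section, gated by a DamageGiven flag, it applies game-state poop damage scaled by the highest multiplier among box-overlapped floors.
; It then becomes a static, upright cone.
; StepIn plays a squish, converts HP into kitty steps up to the allowed count, and shrinks or destroys the poop.
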(event `self.Poop.OnComponentBeginOverlap`
  (params (OverlappedComponent :type "PrimitiveComponent Object Reference") (OtherActor :type "Actor Object Reference") (OtherComp :type "PrimitiveComponent Object Reference") (OtherBodyIndex :type Integer) (bFromSweep :type Boolean) (SweepResult :type "HitResult Structure (by ref)"))
  (bind (_origin _boxextent) (`self.GetActorBounds` true))
  (bind _poop (`self.Poop`))
  (if (`self.DamageGiven`)
    (cast `FloorSection` OtherActor)
    (bind _outactors (`KismetSystemLibrary.BoxOverlapActors` _origin _boxextent (`|MakeArray` "ObjectTypeQuery1" :!type "EObjectTypeQuery Enum") "/Script/KittyCatastrophe.FloorSection"))
    ;[1 1 1] Check all colliding floors and use only the highest damage multiplier.
    (for _array_element _outactors
      (bind _asfloor_section (cast `FloorSection` _array_element))
      (bind _output_get (set `self.DamageMultiplier` (`KismetMathLibrary.FMax` (stale _output_get) (`FloorSection.DAMAGE_MULTIPLIER` _asfloor_section)))))
    ;[1 1 1] Decrease level health.
    (bind _asgame_state (cast `/Game/KittyCatastrophe/Core/GameModes/BP_GameState` (`GameplayStatics.GetGameState`)))
    (`/Game/KittyCatastrophe/Core/GameModes/BP_GameState.DecreaseLevelHealth` _asgame_state (* (`/Game/KittyCatastrophe/Core/GameModes/BP_GameState.POOP_DAMAGE` _asgame_state) (`self.DamageMultiplier`)))
    (set `self.DamageGiven` true)
    (`StaticMeshComponent.SetStaticMesh` _poop "/Engine/BasicShapes/Cone.Cone")
    (`PrimitiveComponent.SetSimulatePhysics` _poop false)
    (`self.K2_SetActorRotation` (struct) true)))

(fn `StepIn`
  (params (KittySteps :type "Integer (by ref)") (AllowedSteps :type Integer))
  (locals (StepsGiven :type Integer))
  (if (`KismetMathLibrary.Conv_IntToBool` AllowedSteps)
    (`GameplayStatics.PlaySoundAtLocation` "/Game/KittyCatastrophe/Characters/Kitty/Sounds/S_Squish_Cue.S_Squish_Cue" (`self.K2_GetActorLocation`) (struct) 1.0 1.0 0.0 null null null)
    (bind _output_get (set `local.StepsGiven` (`KismetMathLibrary.Min` (`self.HP`) AllowedSteps)))
    (`|VariableSetRef` KittySteps (+ KittySteps _output_get))
    (bind _output_get_2 (set `self.HP` (- (stale _output_get_2) _output_get)))
    (if (<= _output_get_2 0)
      (`self.K2_DestroyActor`)
      (else
        ;[1 1 1] TODO: make relative?
        (`self.SetActorScale3D` (`KismetMathLibrary.Conv_DoubleToVector` (/ (`KismetMathLibrary.Conv_IntToDouble` _output_get_2) (`KismetMathLibrary.Conv_IntToDouble` (`self.MAX_HP`)))))))))

(fn `UserConstructionScript`)