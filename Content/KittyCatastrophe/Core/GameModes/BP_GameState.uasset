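; BP_GameState is the game state for Kitty Catastrophe, tracking a shared level health value that starts at its maximum in the construction script.
; DecreaseLevelHealth and IncreaseLevelHealth adjust that value, clamped between zero and MAXLEVELHEALTH.
; A decrease that leaves health at zero calls the Catastrophe event, which only prints a red "CATASTROPHE" message on screen.
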(event `Catastrophe`
  (`KismetSystemLibrary.PrintString` "CATASTROPHE" true true (struct :`R` 1.0 :`A` 1.0) 10.0))

(fn `DecreaseLevelHealth`
  (params (Amount :type "Float (double-precision)" :default 0.0))
  (locals (NewLevelHealth :type "Float (double-precision)"))
  (bind _output_get (set `self.LevelHealth` (`KismetMathLibrary.FMax` (- (stale _output_get) Amount))))
  (if (== _output_get 0.0)
    (`self.Catastrophe`)))

(fn `IncreaseLevelHealth`
  (params (Amount :type "Float (double-precision)"))
  (bind _output_get (set `self.LevelHealth` (`KismetMathLibrary.FMin` (+ (stale _output_get) Amount) (`self.MAX_LEVEL_HEALTH`)))))

(fn `UserConstructionScript`
  (set `self.LevelHealth` (`self.MAX_LEVEL_HEALTH`)))