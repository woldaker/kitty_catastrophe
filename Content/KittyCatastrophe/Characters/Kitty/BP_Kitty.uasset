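; BP_Kitty is the cat character that meows, poops and steps in poop, turning smoothly toward its control rotation.
; A one-second timer counts down PoopTimer, which Feed extends, triggering periodic meows and then Poop, which clears the timer.
; Poop spawns one scaled BP_Poop or, above a food threshold, sprays impulse-driven chunks through a delayed-loop macro.
; PoopFunc is an uncalled, delay-free variant; overlapping poop calls its StepIn with step counts.
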(event `Poop`
  (bind _diarrhea_chunk_scale (`self.DIARRHEA_CHUNK_SCALE`))
  (bind _foodamount (`self.FoodAmount`))
  (bind _returnvalue (`SceneComponent.GetSocketLocation` (`self.SK_Kitty`) "Butt"))
  (bind _returnvalue_2 (`SceneComponent.GetSocketLocation` (`self.SK_Kitty`) "Butt"))
  (if (> _foodamount 0)
    (if (>= _foodamount (`self.DIARRHEA_THRESHOLD`))
      ;[1 1 0] Explosive diarrhea
      (`self.WhileLoopWithDelay` 0.05 (> (`self.FoodAmount`) 0)
        (:`Loop Body`
          (bind _output_get (set `self.FoodAmount` (`KismetMathLibrary.Max` (- (stale _output_get) (`self.DIARRHEA_CHUNK_SIZE`)))))
          (`GameplayStatics.PlaySoundAtLocation` "/Game/KittyCatastrophe/Characters/Kitty/Sounds/S_Poop_Cue.S_Poop_Cue" _returnvalue_2 (struct) 1.0 1.0 0.0 null null null)
          (bind _returnvalue_3 (`|SpawnActorFromClass` "/Game/KittyCatastrophe/Interactables/BP_Poop.BP_Poop_C" (`KismetMathLibrary.MakeTransform` _returnvalue_2 (`KismetMathLibrary.MakeRotator` 0.0 (`self.POOPING_ANGLE_DIARRHEA`)) (`KismetMathLibrary.Conv_DoubleToVector` _diarrhea_chunk_scale)) "AdjustIfPossibleButAlwaysSpawn" "OverrideRootScale" null (`KismetMathLibrary.FTrunc` (* (defaults `/Game/KittyCatastrophe/Interactables/BP_Poop` "/Game/KittyCatastrophe/Interactables/BP_Poop.BP_Poop_C") _diarrhea_chunk_scale)) null))
          (`PrimitiveComponent.AddImpulse` (`/Game/KittyCatastrophe/Interactables/BP_Poop.Poop` _returnvalue_3) (* (`KismetMathLibrary.RandomUnitVectorInConeInDegrees` (`KismetMathLibrary.GreaterGreater_VectorRotator` (* (`self.GetActorForwardVector`) -1) (`KismetMathLibrary.MakeRotator` 0.0 (`self.POOPING_ANGLE_DIARRHEA`))) (`self.DIARRHEA_SPRAY_ANGLE`)) (`self.DIARRHEA_SPRAY_FORCE_`)) "None" false))
        (:`Completed`
          (`self.InvalidatePoopTimer`)))
      (else
        ;[1 1 0] Regular pooping
        (`GameplayStatics.PlaySoundAtLocation` "/Game/KittyCatastrophe/Characters/Kitty/Sounds/S_Poop_Cue.S_Poop_Cue" _returnvalue (struct) 1.0 1.0 0.0 null null null)
        (`|SpawnActorFromClass` "/Game/KittyCatastrophe/Interactables/BP_Poop.BP_Poop_C" (`KismetMathLibrary.MakeTransform` _returnvalue (`KismetMathLibrary.MakeRotator` 0.0 (`self.POOPING_ANGLE`)) (`KismetMathLibrary.Conv_DoubleToVector` (/ (`KismetMathLibrary.Conv_IntToDouble` (`self.FoodAmount`)) (`KismetMathLibrary.Conv_IntToDouble` (`self.DIARRHEA_THRESHOLD`))))) "AdjustIfPossibleButAlwaysSpawn" "OverrideRootScale" null 20 null)
        (set `self.FoodAmount` 0)
        (`self.InvalidatePoopTimer`)))))

(event `self.ReceiveBeginPlay`
  (bind _returnvalue (`KismetSystemLibrary.K2_SetTimer` null "DecrementPoopTimer" 1.0 true)))

(event `InvalidatePoopTimer`
  (`KismetSystemLibrary.K2_ClearAndInvalidateTimerHandle` (stale `self.ReceiveBeginPlay` _returnvalue)))

(event `self.ReceiveTick`
  (params (DeltaSeconds :type "Float (single-precision)"))
  (`self.K2_SetActorRotation` (`KismetMathLibrary.RInterpTo_Constant` (`self.K2_GetActorRotation`) (`self.GetControlRotation`) DeltaSeconds (`self.TURNING_SPEED`))))

(event `self.StepInCollider.OnComponentBeginOverlap`
  (params (OverlappedComponent :type "PrimitiveComponent Object Reference") (OtherActor :type "Actor Object Reference") (OtherComp :type "PrimitiveComponent Object Reference") (OtherBodyIndex :type Integer) (bFromSweep :type Boolean) (SweepResult :type "HitResult Structure (by ref)"))
  (bind _poopsteps (`self.PoopSteps`))
  (bind _asbp_poop (cast `/Game/KittyCatastrophe/Interactables/BP_Poop` OtherActor))
  (`/Game/KittyCatastrophe/Interactables/BP_Poop.StepIn` _asbp_poop _poopsteps (- (`self.MAX_POOP_STEPS`) _poopsteps)))

(fn `DecrementPoopTimer`
  (locals (MeowEveryNSeconds :type Integer :default 5))
  (bind _pooptimer (`self.PoopTimer`))
  (bind _result (`/Engine/EditorBlueprintResources/StandardMacros.DecrementInt` (`self.PoopTimer`))
    (:`  `
      ;[1 1 1] If poop timer hasn't expired, meow every few seconds
      (if (and (> _pooptimer 0) (== (mod _pooptimer (`local.MeowEveryNSeconds`)) 0))
        (`self.Meow`))
      ;[1 1 1] When timer reaches zero, spawn Poop
      (if (not (`KismetMathLibrary.Conv_IntToBool` _result))
        (`self.Poop`)))))

(fn `Feed`
  (params (Amount :type Integer :default 5))
  (returns (AmountEaten :type Integer))
  (locals (AmountFed :type Integer))
  (bind _foodamount (`self.FoodAmount`))
  (bind _max_food_amount (`self.MAX_FOOD_AMOUNT`))
  (if (< _foodamount _max_food_amount)
    (bind _output_get (set `local.AmountFed` (`KismetMathLibrary.Min` (- _max_food_amount _foodamount) Amount)))
    (bind _output_get_2 (set `self.PoopTimer` (+ (stale _output_get_2) (`KismetMathLibrary.Round` (* _output_get (`self.TIME_PER_FOOD_UNIT`)))))))
  (return (`local.AmountFed`)))

(fn `Meow`
  (locals (ThresholdMild :type Integer :default 25) (ThresholdNormal :type Integer :default 15) (ThresholdUrgent :type Integer :default 5) (MeowSound :type "SoundCue Object Reference" :default "SoundCue'/Game/KittyCatastrophe/Characters/Kitty/Sounds/S_Meow_Urgent_Cue.S_Meow_Urgent_Cue'"))
  (`|ExecutionSequence`
    (:`then_0`
      (if (>= (`self.PoopTimer`) (`local.ThresholdMild`))
        (set `local.MeowSound` "/Game/KittyCatastrophe/Characters/Kitty/Sounds/S_Meow_Mild_Cue.S_Meow_Mild_Cue")
        (elif (>= (`self.PoopTimer`) (`local.ThresholdNormal`))
          (set `local.MeowSound` "/Game/KittyCatastrophe/Characters/Kitty/Sounds/S_Meow_Normal_Cue.S_Meow_Normal_Cue"))))
    (:`then_1`
      (`GameplayStatics.PlaySoundAtLocation` (`local.MeowSound`) (`self.K2_GetActorLocation`) (struct) 1.0 1.0 0.0 null null null))))

(fn `PlayWithLure`
  (set `self.Playing` true))

(fn `PoopFunc`
  (locals (POOPING_ANGLE_NORMAL :type "Float (double-precision)" :default -30.0) (POOPING_ANGLE_DIARRHEA :type "Float (double-precision)" :default 15.0) (DiarrheaChunkScale :type "Float (double-precision)") (DIARRHEA_SPRAY_ANGLE :type "Float (double-precision)" :default 30.0) (DIARRHEA_SPRAY_FORCE :type "Float (double-precision)" :default 200.0))
  (bind _diarrheachunkscale (`local.DiarrheaChunkScale`))
  (bind _foodamount (`self.FoodAmount`))
  (bind _returnvalue (`SceneComponent.GetSocketLocation` (`self.SK_Kitty`) "Butt"))
  (bind _returnvalue_2 (`SceneComponent.GetSocketLocation` (`self.SK_Kitty`) "Butt"))
  (if (> _foodamount 0)
    (if (>= _foodamount (`self.DIARRHEA_THRESHOLD`))
      (set `local.DiarrheaChunkScale` (`KismetMathLibrary.FClamp` (/ (`KismetMathLibrary.Conv_IntToDouble` (`self.DIARRHEA_CHUNK_SIZE`)) (`KismetMathLibrary.Conv_IntToDouble` (`self.MAX_FOOD_AMOUNT`)))))
      (while (> (`self.FoodAmount`) 0)
        (bind _output_get (set `self.FoodAmount` (`KismetMathLibrary.Max` (- (stale _output_get) (`self.DIARRHEA_CHUNK_SIZE`)))))
        (`GameplayStatics.PlaySoundAtLocation` "/Game/KittyCatastrophe/Characters/Kitty/Sounds/S_Poop_Cue.S_Poop_Cue" _returnvalue_2 (struct) 1.0 1.0 0.0 null null null)
        (bind _returnvalue_3 (`|SpawnActorFromClass` "/Game/KittyCatastrophe/Interactables/BP_Poop.BP_Poop_C" (`KismetMathLibrary.MakeTransform` _returnvalue_2 (`KismetMathLibrary.MakeRotator` 0.0 (`local.POOPING_ANGLE_DIARRHEA`)) (`KismetMathLibrary.Conv_DoubleToVector` _diarrheachunkscale)) "AlwaysSpawn" "OverrideRootScale" null (`KismetMathLibrary.FTrunc` (* (defaults `/Game/KittyCatastrophe/Interactables/BP_Poop` "/Game/KittyCatastrophe/Interactables/BP_Poop.BP_Poop_C") _diarrheachunkscale)) null))
        (`PrimitiveComponent.AddImpulse` (`/Game/KittyCatastrophe/Interactables/BP_Poop.Poop` _returnvalue_3) (* (`KismetMathLibrary.RandomUnitVectorInConeInDegrees` (`KismetMathLibrary.GreaterGreater_VectorRotator` (* (`self.GetActorForwardVector`) -1) (`KismetMathLibrary.MakeRotator` 0.0 (`local.POOPING_ANGLE_DIARRHEA`))) (`local.DIARRHEA_SPRAY_ANGLE`)) 0.0) "None" false))
      (`self.InvalidatePoopTimer`)
      (else
        (`GameplayStatics.PlaySoundAtLocation` "/Game/KittyCatastrophe/Characters/Kitty/Sounds/S_Poop_Cue.S_Poop_Cue" _returnvalue (struct) 1.0 1.0 0.0 null null null)
        (`|SpawnActorFromClass` "/Game/KittyCatastrophe/Interactables/BP_Poop.BP_Poop_C" (`KismetMathLibrary.MakeTransform` _returnvalue (`KismetMathLibrary.MakeRotator` 0.0 (`local.POOPING_ANGLE_NORMAL`)) (`KismetMathLibrary.Conv_DoubleToVector` (/ (`KismetMathLibrary.Conv_IntToDouble` (`self.FoodAmount`)) (`KismetMathLibrary.Conv_IntToDouble` (`self.DIARRHEA_THRESHOLD`))))) "AdjustIfPossibleButAlwaysSpawn" "OverrideRootScale" null (defaults `/Game/KittyCatastrophe/Interactables/BP_Poop` "/Game/KittyCatastrophe/Interactables/BP_Poop.BP_Poop_C") null)
        (set `self.FoodAmount` 0)
        (`self.InvalidatePoopTimer`)))))

(fn `UserConstructionScript`)